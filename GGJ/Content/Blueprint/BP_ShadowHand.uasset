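; BP_ShadowHand is an actor showing a shadow hand flipbook that travels along a spline in the rope-puller game.
; Every Tick it reads HandLocationRatio from GM_RopePuller, mapping it from spline end to start to set the flipbook's position and rotation, with pitch offset by -90 degrees.
; While the ratio exceeds a small threshold, a DoOnce with a delayed reset replays the hand sound about once a second.
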(event `self.ReceiveTick`
  (params (DeltaSeconds :type "Float (single-precision)"))
  (bind _paperflipbook (`self.PaperFlipbook`))
  (bind _handlocationratio (`/Game/Blueprint/GM_RopePuller.handLocationRatio` (cast `/Game/Blueprint/GM_RopePuller` (`GameplayStatics.GetGameMode`) :!pure true)))
  (`SceneComponent.K2_SetWorldLocation` _paperflipbook (`SplineComponent.GetLocationAtDistanceAlongSpline` (`self.Spline`) (`KismetMathLibrary.Lerp` (`SplineComponent.GetSplineLength` (`self.Spline`)) 0.0 _handlocationratio) "World") false false)
  (`SceneComponent.K2_SetWorldRotation` _paperflipbook (`KismetMathLibrary.MakeRotator` (.roll (`SplineComponent.GetRotationAtDistanceAlongSpline` (`self.Spline`) (`KismetMathLibrary.Lerp` (`SplineComponent.GetSplineLength` (`self.Spline`)) 0.0 _handlocationratio) "World")) (+ (.pitch (`SplineComponent.GetRotationAtDistanceAlongSpline` (`self.Spline`) (`KismetMathLibrary.Lerp` (`SplineComponent.GetSplineLength` (`self.Spline`)) 0.0 _handlocationratio) "World")) -90.0) (.yaw (`SplineComponent.GetRotationAtDistanceAlongSpline` (`self.Spline`) (`KismetMathLibrary.Lerp` (`SplineComponent.GetSplineLength` (`self.Spline`)) 0.0 _handlocationratio) "World"))) false false)
  (if (> _handlocationratio 0.2)
    (`/Engine/EditorBlueprintResources/StandardMacros.DoOnce` false :!label _label
      (:`Completed`
        (`GameplayStatics.PlaySound2D` "/Game/Sound/Hands/S_Black_HandsShorts.S_Black_HandsShorts" 1.0 1.0 0.0 null null)
        (`KismetSystemLibrary.Delay` 1.0)
        (goto _label :!via `Reset`)))))

(fn `UserConstructionScript`)