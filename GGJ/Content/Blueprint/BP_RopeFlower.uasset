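; Tug-of-war rope actor that spawns a flower and a fire effect at its center, with Light and Shadow players pulling the flower.
; Each tick it reads GM_RopePuller's pull flags to slide the flower, frame-rate compensated, within RopeLength, and reports its side to UpdateIntensity.
; Game mode state also toggles the fire and immunity plane, and RopeStatus swaps wear textures on a dynamic material created in construction.
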(event `self.ReceiveBeginPlay`
  (bind _returnvalue (`KismetMathLibrary.MakeTransform` (`KismetMathLibrary.MakeVector` (+ (.x (`SceneComponent.K2_GetComponentLocation` (`self.Rope`))) -50.0) (.y (`SceneComponent.K2_GetComponentLocation` (`self.Rope`))) (+ (.z (`SceneComponent.K2_GetComponentLocation` (`self.Rope`))) 20.0)) (struct :`Yaw` 90.0)))
  ;[1 1 1] Spawn Flower at center
  (bind _returnvalue_2 (`|SpawnActorFromClass` "/Game/Blueprint/Flower/BP_Flower.BP_Flower_C" _returnvalue "AlwaysSpawn" "OverrideRootScale" null null))
  (bind _returnvalue_3 (`|SpawnActorFromClass` "/Script/Niagara.NiagaraActor" _returnvalue "Undefined" "OverrideRootScale" null null))
  (bind _output_get (set `self.ParticuleSystem` _returnvalue_3))
  (`NiagaraComponent.SetAsset` (`NiagaraActor.NiagaraComponent` _output_get) "/Game/Particules/FX_Fire.FX_Fire" true)
  (set `self.flowerREF` _returnvalue_2)
  (set `self.gamemodeREF` (cast `/Game/Blueprint/GM_RopePuller` (`GameplayStatics.GetGameMode`) :!pure true))
  (`self.Update Rope Texture`))

(event `self.ReceiveTick`
  (params (DeltaSeconds :type "Float (single-precision)"))
  (bind _niagaracomponent (`NiagaraActor.NiagaraComponent` (`self.ParticuleSystem`)))
  ;[1 1 1] Controls on speed (FPS) are each inside those functions
  (`self.Pull Flower`)
  (`/Game/Blueprint/GM_RopePuller.updateIntensity` (`self.gamemodeREF`) (< (.y (`self.K2_GetActorLocation` (`self.flowerREF`))) 0.0))
  (`self.Update Rope Texture`)
  (if (`/Game/Blueprint/GM_RopePuller.isBurning?` (`self.gamemodeREF`))
    (`SceneComponent.SetVisibility` _niagaracomponent true false)
    (else
      (`SceneComponent.SetVisibility` _niagaracomponent false false))))

(fn `Pull Flower`
  (locals (pullForceValue :type "Float (double-precision)") (glideDistance :type "Float (double-precision)" :default 10.0) (newLocation :type "Vector Structure"))
  (bind _flowerref (`self.flowerREF`))
  (bind _gamemoderef (`self.gamemodeREF`))
  (bind _islightpulling_ (`/Game/Blueprint/GM_RopePuller.isLightPulling?` _gamemoderef))
  (bind _flowerspeed (`/Game/Blueprint/GM_RopePuller.flowerSpeed` (cast `/Game/Blueprint/GM_RopePuller` (`GameplayStatics.GetGameMode`) :!pure true)))
  (bind _returnvalue (+ (.y (`self.K2_GetActorLocation` _flowerref)) (* (`local.pullForceValue`) (* (`GameplayStatics.GetWorldDeltaSeconds`) 60.0))))
  (if (`KismetMathLibrary.BooleanNOR` (`/Game/Blueprint/GM_RopePuller.isLightPulling?` _gamemoderef) (`/Game/Blueprint/GM_RopePuller.isShadowPulling?` _gamemoderef))
    ;[1 1 1] Decide direction
    (set `local.pullForceValue` 0.0 :!label _label)
    (elif (and _islightpulling_ (`/Game/Blueprint/GM_RopePuller.isShadowPulling?` _gamemoderef))
      (goto _label)
      (elif _islightpulling_
        (set `local.pullForceValue` (* _flowerspeed -1.0)) ; To the left
        (else
          (set `local.pullForceValue` _flowerspeed) ; To the right
        ))))
  ;[1 1 1] Move to pull direction
  (if (not (>= (`KismetMathLibrary.Abs` _returnvalue) (/ (* 100 (`self.ropeLength`)) 2.0)))
    (bind _output_get (set `local.newLocation` (`KismetMathLibrary.MakeVector` (.x (`self.K2_GetActorLocation` _flowerref)) _returnvalue (.z (`self.K2_GetActorLocation` _flowerref))))) ; Used for Gliding
    (`self.K2_SetActorLocation` _flowerref _output_get false false)))

(fn `Update Rope Texture`
  (bind _gamemoderef (`self.gamemodeREF`))
  (bind _ropestatus (`/Game/Blueprint/GM_RopePuller.ropeStatus` _gamemoderef))
  (`SceneComponent.SetVisibility` (`self.Plane`) (`/Game/Blueprint/GM_RopePuller.isImmuneToDommage?` _gamemoderef) false)
  (if (< _ropestatus 1.0)
    (`MaterialInstanceDynamic.SetTextureParameterValue` (`self.dynamicMatREF`) "Texture" "/Game/Texture/Ropes/T_Corde_6.T_Corde_6")
    (elif (< _ropestatus 20.0)
      (`MaterialInstanceDynamic.SetTextureParameterValue` (`self.dynamicMatREF`) "Texture" "/Game/Texture/Ropes/T_Corde_5.T_Corde_5")
      (elif (< _ropestatus 40.0)
        (`MaterialInstanceDynamic.SetTextureParameterValue` (`self.dynamicMatREF`) "Texture" "/Game/Texture/Ropes/T_Corde_4.T_Corde_4")
        (elif (< _ropestatus 60.0)
          (`MaterialInstanceDynamic.SetTextureParameterValue` (`self.dynamicMatREF`) "Texture" "/Game/Texture/Ropes/T_Corde_3.T_Corde_3")
          (elif (< _ropestatus 80.0)
            (`MaterialInstanceDynamic.SetTextureParameterValue` (`self.dynamicMatREF`) "Texture" "/Game/Texture/Ropes/T_Corde_2.T_Corde_2")
            (else
              (`MaterialInstanceDynamic.SetTextureParameterValue` (`self.dynamicMatREF`) "Texture" "/Game/Texture/Ropes/T_Corde_1.T_Corde_1"))))))))

(fn `UserConstructionScript`
  (`SceneComponent.SetRelativeScale3D` (`self.Rope`) (`KismetMathLibrary.MakeVector` (`self.ropeLength`) 0.5 1.0))
  (bind _returnvalue (`KismetMaterialLibrary.CreateDynamicMaterialInstance` "/Game/Material/M_Rope.M_Rope"))
  (bind _output_get (set `self.dynamicMatREF` _returnvalue))
  (`MaterialInstanceDynamic.SetTextureParameterValue` _output_get "Texture" "/Game/Texture/Ropes/T_Corde_1.T_Corde_1")
  (`PrimitiveComponent.SetMaterial` (`self.Rope`) 0 _output_get))