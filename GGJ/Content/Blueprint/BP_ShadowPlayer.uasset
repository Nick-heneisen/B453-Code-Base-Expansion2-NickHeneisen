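; BP_ShadowPlayer is the shadow-side player in a rope-pulling game, shown as a Paper2D girl sprite.
; Pull input sets the shadow pulling flag on GM_RopePuller and swaps the flipbook between pull and idle.
; Skill input, allowed only with a charge and low enough light intensity, calls the game mode's ShadowSkill, spends the charge, removes a UI shard and plays a sound.
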(event `InputAction|Pull`
  (params (Key :type "Key Structure"))
  (bind _asgm_rope_puller (cast `/Game/Blueprint/GM_RopePuller` (`GameplayStatics.GetGameMode`) :!pure true))
  (:`Pressed`
    (set `/Game/Blueprint/GM_RopePuller.isShadowPulling?` true _asgm_rope_puller))
  (:`Released`
    (set `/Game/Blueprint/GM_RopePuller.isShadowPulling?` false _asgm_rope_puller)))

(event `InputAction|Skill`
  (params (Key :type "Key Structure"))
  (bind _asgm_rope_puller (cast `/Game/Blueprint/GM_RopePuller` (`GameplayStatics.GetGameMode`) :!pure true))
  (:`Pressed`
    (if (and (`self.hasCharge?`) (<= (`/Game/Blueprint/GM_RopePuller.lightIntensity` _asgm_rope_puller) 50.0))
      (`/Game/Blueprint/GM_RopePuller.ShadowSkill` _asgm_rope_puller (`self.skillDuration`))
      (set `self.hasCharge?` false)
      (`/Game/Blueprint/Widget/W_GameWidget.RemoveShadowShard` (`self.UIRef`))
      (`GameplayStatics.PlaySound2D` "/Game/Sound/Activation_compétence/270409__littlerobotsoundfactory__spell-00.270409__littlerobotsoundfactory__spell-00" 1.0 1.0 0.0 null null))))

(event `InputAction|Pull`
  (params (Key :type "Key Structure"))
  ;[1 1 1] Change animation
  (:`Pressed`
    (`PaperFlipbookComponent.SetFlipbook` (`self.PaperFlipbook`) "/Game/Sprite/Sprite_Girl_Pull/T_Girl_Pull.T_Girl_Pull"))
  (:`Released`
    (`PaperFlipbookComponent.SetFlipbook` (`self.PaperFlipbook`) "/Game/Sprite/Sprite_Girl_Idle/FPB_Girl_Idle.FPB_Girl_Idle")))

(fn `UserConstructionScript`
  (`parent.UserConstructionScript`))