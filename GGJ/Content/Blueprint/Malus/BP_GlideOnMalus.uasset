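; BP_GlideOnMalus is a malus pickup that makes play slippery by triggering a glide effect when a flower touches it.
; On collision overlap with a BP_Flower, it tells the flower to add a slow part and asks GM_RopePuller to run Glide for the malus duration.
; It then plays a swoop sound and destroys itself.
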(event `self.Collision.OnComponentBeginOverlap`
  (params (OverlappedComponent :type "PrimitiveComponent Object Reference") (OtherActor :type "Actor Object Reference") (OtherComp :type "PrimitiveComponent Object Reference") (OtherBodyIndex :type Integer) (bFromSweep :type Boolean) (SweepResult :type "HitResult Structure (by ref)"))
  (bind (_asbp_flower _bsuccess) (cast `/Game/Blueprint/Flower/BP_Flower` OtherActor :!pure true))
  (if _bsuccess
    (`/Game/Blueprint/Flower/BP_Flower.addSlowPart` _asbp_flower)
    (`/Game/Blueprint/GM_RopePuller.Glide` (cast `/Game/Blueprint/GM_RopePuller` (`GameplayStatics.GetGameMode`) :!pure true) (`self.malusDuration`))
    (`GameplayStatics.PlaySound2D` "/Game/Sound/Malus/174764__yottasounds__swoop-007.174764__yottasounds__swoop-007" 1.0 1.0 0.0 null null)
    (`self.K2_DestroyActor`)))

(fn `UserConstructionScript`
  (`parent.UserConstructionScript`))