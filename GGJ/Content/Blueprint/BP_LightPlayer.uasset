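; Player Blueprint for the light side of a rope-pulling game, with a Paper2D flipbook character.
; Pull input toggles the light-pulling flag on GM_RopePuller and swaps between pull and idle flipbooks.
; Skill input spends a single charge when the game mode's light intensity is high enough, triggering LightSkill, flower speed particles and a UI charge update.
; Enchant and disenchant sounds bracket the skill's duration.
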(event `self.ReceiveBeginPlay`
  (`self.EnableInput` (`GameplayStatics.GetPlayerController` 0)))

(event `InputAction|Pull`
  (params (Key :type "Key Structure"))
  (bind _asgm_rope_puller (cast `/Game/Blueprint/GM_RopePuller` (`GameplayStatics.GetGameMode`) :!pure true))
  (:`Pressed`
    (set `/Game/Blueprint/GM_RopePuller.isLightPulling?` true _asgm_rope_puller))
  (:`Released`
    (set `/Game/Blueprint/GM_RopePuller.isLightPulling?` false _asgm_rope_puller)))

(event `InputAction|Skill`
  (params (Key :type "Key Structure"))
  (bind _asgm_rope_puller (cast `/Game/Blueprint/GM_RopePuller` (`GameplayStatics.GetGameMode`) :!pure true))
  ;[1 1 1] Light skill
  (:`Pressed`
    (if (and (`self.hasCharge?`) (>= (`/Game/Blueprint/GM_RopePuller.lightIntensity` _asgm_rope_puller) 50.0))
      (`/Game/Blueprint/GM_RopePuller.LightSkill` _asgm_rope_puller (`self.skillDuration`))
      (set `self.hasCharge?` false)
      (`GameplayStatics.PlaySound2D` "/Game/Sound/Activation_compétence/202147__qubodup__enchant.202147__qubodup__enchant" 1.0 1.0 0.0 null null)
      (`/Game/Blueprint/Flower/BP_Flower.addSpeedParticule` (`self.FlowerREF`))
      (`/Game/Blueprint/Widget/W_GameWidget.RemoveLightCharge` (`self.UIRef`))
      (`KismetSystemLibrary.Delay` (`self.skillDuration`))
      (`GameplayStatics.PlaySound2D` "/Game/Sound/Activation_compétence/202148__qubodup__disenchant.202148__qubodup__disenchant" 1.0 1.0 0.0 null null))))

(event `InputAction|Pull`
  (params (Key :type "Key Structure"))
  (:`Pressed`
    (`PaperFlipbookComponent.SetFlipbook` (`self.PaperFlipbook`) "/Game/Sprite/T_Man_Pull/PFB_Man_Pull.PFB_Man_Pull"))
  (:`Released`
    (`PaperFlipbookComponent.SetFlipbook` (`self.PaperFlipbook`) "/Game/Sprite/Sprite_Man_Idle/FPB_Man_Idle.FPB_Man_Idle")))

(fn `UserConstructionScript`
  (`parent.UserConstructionScript`))